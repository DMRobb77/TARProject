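; Side-scrolling player character that moves along the Y axis and jumps with height affected by how long the button is held.
; BeginPlay spawns a separate camera actor as the view target, offset from the CameraBoom.
; Tick eases that camera after the boom, flipping its horizontal offset by the pawn's yaw sign to follow facing.
; Experimental sprint speed logic is present but disconnected, and the CanJumpInternal override only returns the parent result.
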(event `InputAction|Jump`
  ;[1 1 1] Jump Affected by Time Button Held
  (:`Pressed`
    (`self.Jump`))
  (:`Released`
    (`self.StopJumping`)))

(event `InputAxis|MoveRight`
  (params (AxisValue :type "Float (single-precision)"))
  (`self.AddMovementInput` (0.0 -1.0 0.0) AxisValue))

(event `Key|LeftShift`
  ;[1 1 1] Running (Experimental
)

(event `self.ReceiveTick`
  (params (DeltaSeconds :type "Float (single-precision)"))
  (if (>= (`KismetMathLibrary.FFloor` (.yaw (`self.K2_GetActorRotation` (`GameplayStatics.GetPlayerPawn` 0)))) 0)
    (set `self.CameraOffsetY` 180.0)
    (else
      (set `self.CameraOffsetY` -180.0)))
  (`self.SetActorTransform` (stale `self.ReceiveBeginPlay` _returnvalue) (`KismetMathLibrary.TInterpTo` (`self.GetTransform` (stale `self.ReceiveBeginPlay` _returnvalue)) (`KismetMathLibrary.MakeTransform` (`KismetMathLibrary.MakeVector` (+ (.x (.location (`SceneComponent.K2_GetComponentToWorld` (`self.CameraBoom`)))) 1128.0) (+ (.y (.location (`SceneComponent.K2_GetComponentToWorld` (`self.CameraBoom`)))) (`self.CameraOffsetY`)) (+ (.z (.location (`SceneComponent.K2_GetComponentToWorld` (`self.CameraBoom`)))) 110.0)) (.rotation (`SceneComponent.K2_GetComponentToWorld` (`self.CameraBoom`))) (.scale (`SceneComponent.K2_GetComponentToWorld` (`self.CameraBoom`)))) DeltaSeconds 6.0) false))

(event `self.ReceiveBeginPlay`
  (bind _returnvalue (`|SpawnActorFromClass` "/Script/Engine.CameraActor" (`KismetMathLibrary.MakeTransform` (`KismetMathLibrary.MakeVector` (+ (.x (.location (`SceneComponent.K2_GetComponentToWorld` (`self.CameraBoom`)))) 1128.0) (+ (.y (.location (`SceneComponent.K2_GetComponentToWorld` (`self.CameraBoom`)))) (`self.CameraOffsetY`)) (+ (.z (.location (`SceneComponent.K2_GetComponentToWorld` (`self.CameraBoom`)))) 110.0)) (.rotation (`SceneComponent.K2_GetComponentToWorld` (`self.CameraBoom`))) (.scale (`SceneComponent.K2_GetComponentToWorld` (`self.CameraBoom`))))))
  (set `CameraComponent.bConstrainAspectRatio` false (`CameraActor.CameraComponent` _returnvalue))
  (`PlayerController.SetViewTargetWithBlend` (`GameplayStatics.GetPlayerController` 0) _returnvalue 0.0 "VTBlend_Linear" 0.0 false))

(fn `CanJumpInternal`
  (returns (ReturnValue :type Boolean))
  (bind _returnvalue (`parent.CanJumpInternal`))
  (return _returnvalue))

(fn `UserConstructionScript`)